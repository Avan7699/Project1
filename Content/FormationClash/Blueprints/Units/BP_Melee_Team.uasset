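; Melee team unit for Formation Clash, built as a formation of five cells that share a Combat component and each have a health bar widget.
; BeginPlay tints Cell1 to Cell4 blue or red by TeamID through dynamic materials, leaving the Cylinder (cell 0) untinted.
; Combat events update bars by cell index, though cells 3 and 4 always show zero, and hide a dead cell's mesh and bar.
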(event `self.ReceiveBeginPlay`
  (bind _returnvalue (select `int` (`CombatComponent.TeamID` (`self.Combat`)) :`0` (struct :`B` 0.697391 :`A` 1.0) :`1` (struct :`R` 0.801739 :`A` 1.0) :!type "LinearColor Structure"))
  (`parent.ReceiveBeginPlay`)
  (bind _returnvalue_2 (`PrimitiveComponent.CreateDynamicMaterialInstance` (`self.Cell1`) 0 null "None"))
  (`MaterialInstanceDynamic.SetVectorParameterValue` _returnvalue_2 "TeamColor" _returnvalue)
  (bind _returnvalue_3 (`PrimitiveComponent.CreateDynamicMaterialInstance` (`self.Cell2`) 0 null "None"))
  (`MaterialInstanceDynamic.SetVectorParameterValue` _returnvalue_3 "TeamColor" _returnvalue)
  (bind _returnvalue_4 (`PrimitiveComponent.CreateDynamicMaterialInstance` (`self.Cell3`) 0 null "None"))
  (`MaterialInstanceDynamic.SetVectorParameterValue` _returnvalue_4 "TeamColor" _returnvalue)
  (bind _returnvalue_5 (`PrimitiveComponent.CreateDynamicMaterialInstance` (`self.Cell4`) 0 null "None"))
  (`MaterialInstanceDynamic.SetVectorParameterValue` _returnvalue_5 "TeamColor" _returnvalue))

(event `self.Combat.OnCellHealthChanged`
  (params (CellIndex :type Integer) (NewCellHealthPercent :type "Float (single-precision)") (CellsAlive :type Integer))
  (switch `int` CellIndex
    (:`0`
      (bind _aswbp_health_bar (cast `/Game/FormationClash/Blueprints/WBP_HealthBar` (`WidgetComponent.GetWidget` (`self.CellHP0`))))
      (`ProgressBar.SetPercent` (`/Game/FormationClash/Blueprints/WBP_HealthBar.HealthBar` _aswbp_health_bar) NewCellHealthPercent))
    (:`1`
      (bind _aswbp_health_bar_2 (cast `/Game/FormationClash/Blueprints/WBP_HealthBar` (`WidgetComponent.GetWidget` (`self.CellHP1`))))
      (`ProgressBar.SetPercent` (`/Game/FormationClash/Blueprints/WBP_HealthBar.HealthBar` _aswbp_health_bar_2) NewCellHealthPercent))
    (:`2`
      (bind _aswbp_health_bar_3 (cast `/Game/FormationClash/Blueprints/WBP_HealthBar` (`WidgetComponent.GetWidget` (`self.CellHP2`))))
      (`ProgressBar.SetPercent` (`/Game/FormationClash/Blueprints/WBP_HealthBar.HealthBar` _aswbp_health_bar_3) NewCellHealthPercent))
    (:`3`
      (bind _aswbp_health_bar_4 (cast `/Game/FormationClash/Blueprints/WBP_HealthBar` (`WidgetComponent.GetWidget` (`self.CellHP3`))))
      (`ProgressBar.SetPercent` (`/Game/FormationClash/Blueprints/WBP_HealthBar.HealthBar` _aswbp_health_bar_4) 0.0))
    (:`4`
      (bind _aswbp_health_bar_5 (cast `/Game/FormationClash/Blueprints/WBP_HealthBar` (`WidgetComponent.GetWidget` (`self.CellHP4`))))
      (`ProgressBar.SetPercent` (`/Game/FormationClash/Blueprints/WBP_HealthBar.HealthBar` _aswbp_health_bar_5) 0.0))))

(event `self.Combat.OnCellDeath`
  (params (CellIndex :type Integer) (CellsRemaining :type Integer))
  (switch `int` CellIndex
    (:`0`
      (`SceneComponent.SetVisibility` (`self.Cylinder`) false false)
      (`SceneComponent.SetVisibility` (`self.CellHP0`) false false))
    (:`1`
      (`SceneComponent.SetVisibility` (`self.Cell1`) false false)
      (`SceneComponent.SetVisibility` (`self.CellHP1`) false false))
    (:`2`
      (`SceneComponent.SetVisibility` (`self.Cell2`) false false)
      (`SceneComponent.SetVisibility` (`self.CellHP2`) false false))
    (:`3`
      (`SceneComponent.SetVisibility` (`self.Cell3`) false false)
      (`SceneComponent.SetVisibility` (`self.CellHP3`) false false))
    (:`4`
      (`SceneComponent.SetVisibility` (`self.Cell4`) false false)
      (`SceneComponent.SetVisibility` (`self.CellHP4`) false false))))

(fn `UserConstructionScript`
  (`parent.UserConstructionScript`))