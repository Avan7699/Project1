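; Base unit actor for FormationClash that adds team visuals, projectile firing, health display and death cleanup around its Combat component.
; On BeginPlay a dynamic material instance tints the cylinder mesh by team ID.
; FireProjectile_BP spawns the default projectile at the actor's location with zero rotation when Combat allows an attack.
; Combat events drive the widget health bar and, on death, disable collision and set a short lifespan before removal.
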(event `self.ReceiveBeginPlay`
  (bind _returnvalue (`PrimitiveComponent.CreateDynamicMaterialInstance` (`self.Cylinder`) 0 null "None"))
  (`MaterialInstanceDynamic.SetVectorParameterValue` _returnvalue "TeamColor" (select `int` (`CombatComponent.TeamID` (`self.Combat`)) :`0` (struct :`B` 0.697391 :`A` 1.0) :`1` (struct :`R` 0.801739 :`A` 1.0) :!type "LinearColor Structure")))

(event `Fire Projectile_BP`
  (if (`CombatComponent.bCanAttack` (`self.Combat`))
    (`|SpawnActorFromClass` "/Game/FormationClash/Blueprints/BP_Projectile_Default.BP_Projectile_Default_C" (`KismetMathLibrary.MakeTransform` (`self.K2_GetActorLocation`)) "AlwaysSpawn" "MultiplyWithRoot" null null)))

(event `self.Combat.OnUnitDeath`
  (`self.SetActorEnableCollision` false)
  (`self.SetLifeSpan` 2.0))

(event `self.Combat.OnHealthChanged`
  (params (NewHealthPercent :type "Float (single-precision)"))
  (bind _aswbp_health_bar (cast `/Game/FormationClash/Blueprints/WBP_HealthBar` (`WidgetComponent.GetWidget` (`self.Widget`))))
  (`ProgressBar.SetPercent` (`/Game/FormationClash/Blueprints/WBP_HealthBar.HealthBar` _aswbp_health_bar) NewHealthPercent))

(fn `UserConstructionScript`)